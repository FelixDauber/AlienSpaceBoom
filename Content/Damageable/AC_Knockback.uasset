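; Actor component that pushes its owner away from a hit point when knockback is triggered.
; On BeginPlay it caches the first PrimitiveComponent found on the owner.
; DoKnockback applies a mass-dependent impulse to that component along the normalized direction from the hit point to the component's world location, scaled by ImpulseAmount.
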(event EventDoKnockback
  (params (HitPoint :type Vector :default "0, 0, 0"))
  (Physics|AddImpulse (Variables|Default|GetPrimitive%20Component) (* (Math|Vector|Normalize (- (Transformation|GetWorldLocation (Variables|Default|GetPrimitive%20Component)) HitPoint)) (Variables|Default|GetImpulseAmount)) "None" false))

(event EventBeginPlay
  (Variables|Default|SetPrimitive%20Component (Actor|GetComponentbyClass (Components|GetOwner) "/Script/Engine.PrimitiveComponent")))